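; BP_Disable is a field actor that applies a persistent disable-threshold physics field within a box volume.
; On BeginPlay it clears existing persistent fields, then registers a box falloff at the configurable FieldMagnitude with no falloff.
; A culling field using a second box falloff on the same Box transform culls the effect outside that volume.
; The construction script resets the field system.
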(event `self.ReceiveBeginPlay`
  (bind _fieldsystemcomponent (`self.FieldSystemComponent`))
  (`FieldSystemComponent.RemovePersistentFields` _fieldsystemcomponent)
  (`FieldSystemComponent.AddPersistentField` _fieldsystemcomponent true "Field_DisableThreshold" null (`CullingField.SetCullingField` (`self.CullingField`) (`BoxFalloff.SetBoxFalloff` (`self.BoxCull`) 1.0 0.0 1.0 1.0 (`SceneComponent.K2_GetComponentToWorld` (`self.Box`)) "Field_FallOff_None") (`BoxFalloff.SetBoxFalloff` (`self.BoxFalloff`) (`self.Field Magnitude`) 1.0 1.0 1.0 (`SceneComponent.K2_GetComponentToWorld` (`self.Box`)) "Field_FallOff_None") "Field_Culling_Outside")))

(fn `UserConstructionScript`
  (`FieldSystemComponent.ResetFieldSystem` (`self.FieldSystemComponent`)))