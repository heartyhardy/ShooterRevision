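; Chaos field actor that breaks Geometry Collection destructibles with a one-shot strain burst shortly after BeginPlay.
; After a short random delay, it clears persistent fields and applies external cluster strain through an inverse radial falloff sized and centered by its Sphere component.
; It then applies a radial vector from the same center as internal cluster strain, with no falloff or radius limit.
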(event `self.ReceiveBeginPlay`
  (bind _sphere (`self.Sphere`))
  (bind _fieldsystemcomponent (`self.FieldSystemComponent`))
  (bind _returnvalue (`SceneComponent.K2_GetComponentLocation` _sphere))
  (`KismetSystemLibrary.Delay` (`KismetMathLibrary.RandomFloatInRange` 1.0 2.0))
  (`FieldSystemComponent.RemovePersistentFields` (`self.FieldSystemComponent`))
  (`FieldSystemComponent.ApplyPhysicsField` _fieldsystemcomponent true "Field_ExternalClusterStrain" null (`RadialFalloff.SetRadialFalloff` (`self.RadialFalloff`) (`self.Main Force`) 0.0 1.0 0.0 (`SphereComponent.GetScaledSphereRadius` _sphere) _returnvalue "Field_Falloff_Inverse"))
  (`FieldSystemComponent.ApplyPhysicsField` _fieldsystemcomponent true "Field_InternalClusterStrain" null (`RadialVector.SetRadialVector` (`self.RadialVector`) (`self.Radial Force`) _returnvalue)))

(fn `UserConstructionScript`)